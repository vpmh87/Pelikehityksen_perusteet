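; Candy is a collectible actor that the player picks up by touch and that recycles itself instead of being destroyed.
; On overlap, it passes the other actor's object name to checks for the player character and the respawn trigger.
; A player hit fires the CandyCollectedED dispatcher with the candy's Value.
; Either hit then resets position, scale and value through helper functions not defined in this graph.
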(event EventBeginPlay)

(event Collision|EventActorBeginOverlap
  (params (OtherActor :type Actor%20Object%20Reference))
  (bind _returnvalue (Utilities|GetObjectName OtherActor))
  ;[1 1 1] Collision check on player character
  (bind _hitresult (CallFunction|CheckCharacterHit _returnvalue))
  (if _hitresult
    ;[1 1 1] Candy collected. ED to send.
    (Default|CallCandyCollectedED (Variables|Default|GetValue))
    ;[1 1 1] Reset candy scale and value
    (CallFunction|ResetPosition :!label _label)
    (CallFunction|ResetScaleandValue)
    (else
      ;[1 1 1] If collision hit is not player character, check if hit is on respawntrigger
      (bind _hitresult_2 (CallFunction|CheckRespawnHit _returnvalue))
      (if _hitresult_2
        (goto _label)))))

(event EventTick
  (params (DeltaSeconds :type Float%20%28single-precision%29))
  (|CallParentFunction 0.0))

(fn ConstructionScript)